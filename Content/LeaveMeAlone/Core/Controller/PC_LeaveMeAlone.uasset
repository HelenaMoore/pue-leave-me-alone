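; Player controller for LeaveMeAlone that handles the pause menu and the death screen.
; The Pause input, if not already paused, pauses the game, shows WBP_Pause in UI-only input with the cursor, and stops the pawn's LMAWeaponComponent firing.
; The Death event waits briefly, then pauses the game and shows WBP_DeathScreen with the same UI-only input and cursor.
; OnPause is only set here, never cleared.
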(event `self.ReceiveBeginPlay`)

(event `self.ReceiveTick`
  (params (DeltaSeconds :type "Float (single-precision)")))

(event `InputAction|Pause`
  (params (Key :type "Key Structure"))
  (:`Pressed`
    (if (not (`self.OnPause`))
      (set `self.OnPause` true)
      (`|ExecutionSequence`
        (:`then_0`
          (`GameplayStatics.SetGamePaused` true)
          (bind _returnvalue (`|CreateWidget` "/Game/LeaveMeAlone/Widgets/UI/WBP_Pause.WBP_Pause_C"))
          (bind _output_get (set `self.PauseWidget` _returnvalue))
          (`UserWidget.AddToViewport` _output_get 0)
          (`WidgetBlueprintLibrary.SetInputMode_UIOnlyEx` self _output_get)
          (set `self.bShowMouseCursor` true))
        (:`then_1`
          (`LMAWeaponComponent.StopFire` (`self.GetComponentByClass` (`GameplayStatics.GetPlayerPawn` 0) "/Script/LeaveMeAlone.LMAWeaponComponent")))))))

(event `Death`
  (`KismetSystemLibrary.Delay` 2.0)
  (`GameplayStatics.SetGamePaused` true)
  (bind _returnvalue (`|CreateWidget` "/Game/LeaveMeAlone/Widgets/UI/WBP_DeathScreen.WBP_DeathScreen_C"))
  (bind _output_get (set `self.DeathScreenWidget` _returnvalue))
  (`UserWidget.AddToViewport` _output_get 0)
  (`WidgetBlueprintLibrary.SetInputMode_UIOnlyEx` self _output_get)
  (set `self.bShowMouseCursor` true))

(fn `UserConstructionScript`)