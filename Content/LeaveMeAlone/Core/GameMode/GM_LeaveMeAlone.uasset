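; LeaveMeAlone game mode that runs the match countdown and ends the game when time runs out.
; A looping one-second timer started on BeginPlay decrements GameTime.
; At zero it clears the timer, pauses the game and shows the WBP_GameOver widget, switching the PC_LeaveMeAlone player controller to UI-only input with a visible cursor.
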(event `self.ReceiveBeginPlay`
  (bind _returnvalue (`KismetSystemLibrary.K2_SetTimerDelegate` (delegate `CustomEvent`) 1.0 true))
  (set `self.Game Timer Handle` _returnvalue))

(event `CustomEvent`
  (bind _output_get (set `self.Game Time` (- (`self.Game Time`) 1)))
  (if (== _output_get 0)
    (`|ExecutionSequence`
      (:`then_0`
        (`KismetSystemLibrary.K2_ClearAndInvalidateTimerHandle` (`self.Game Timer Handle`)))
      (:`then_1`
        (`GameplayStatics.SetGamePaused` true)
        (bind _aspc_leave_me_alone (cast `/Game/LeaveMeAlone/Core/Controller/PC_LeaveMeAlone` (`GameplayStatics.GetPlayerController` 0)))
        (bind _returnvalue (`|CreateWidget` "/Game/LeaveMeAlone/Widgets/UI/WBP_GameOver.WBP_GameOver_C"))
        (bind _output_get_2 (set `self.GameOverWidget` _returnvalue))
        (`UserWidget.AddToViewport` _output_get_2 0)
        (`WidgetBlueprintLibrary.SetInputMode_UIOnlyEx` _aspc_leave_me_alone _output_get_2)
        (set `PlayerController.bShowMouseCursor` true _aspc_leave_me_alone)))))

(fn `UserConstructionScript`)